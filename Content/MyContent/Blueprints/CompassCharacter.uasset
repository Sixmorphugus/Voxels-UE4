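; CompassCharacter is a player character Blueprint that moves along fixed world axes and jumps.
; MoveX drives movement along world Y and MoveY along world X, independent of camera or actor facing, while the Jump input triggers a jump.
; Each tick, the camera is placed behind the actor along its own forward vector, at a distance proportional to the viewport's width.
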(event `self.ReceiveTick`
  (params (DeltaSeconds :type "Float (single-precision)"))
  (bind _camera (`self.Camera`))
  (`SceneComponent.K2_SetWorldLocation` _camera (+ (* (* (`SceneComponent.GetForwardVector` _camera) (`KismetMathLibrary.BreakVector2D` (`WidgetLayoutLibrary.GetViewportSize`))) (/ -28.0 2.0)) (`self.K2_GetActorLocation`)) false false))

(event `InputAxis|MoveX`
  (params (AxisValue :type "Float (single-precision)"))
  (`self.AddMovementInput` (0.0 1.0 0.0) AxisValue))

(event `InputAxis|MoveY`
  (params (AxisValue :type "Float (single-precision)"))
  (`self.AddMovementInput` (1.0 0.0 0.0) AxisValue))

(event `InputAction|Jump`
  (params (Key :type "Key Structure" :default "AnyKey"))
  (:`Pressed`
    (`self.Jump`)))

(fn `UserConstructionScript`)